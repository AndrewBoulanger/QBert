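; Base enemy Blueprint that lands on actors tagged Cube, with a fixed rotation set at construction.
; Overlapping a cube stops falling and plays BallJump; leaving it clears the overlap flag.
; A double-speed JumpTimeline is set up to lerp hops left or right and start falling when one ends off a cube, but nothing here starts it.
; CheckIfFalling is an empty stub.
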(event EventBeginPlay
  (bind _output_get (Variables|Default|SetTimeline (Variables|Default|GetJumpTimeline)))
  (Components|Timeline|SetPlayRate _output_get 2.0))

(event Collision|EventActorBeginOverlap
  (params (OtherActor :type Actor%20Object%20Reference))
  (if (Actor|ActorHasTag OtherActor "Cube")
    (Variables|Default|SetIsOverlapping true)
    (Class|BaseEnemy|StopFalling)
    (Audio|Components|Audio|Play (Variables|Default|GetBallJump) 0.0)))

(event Collision|EventActorEndOverlap
  (params (OtherActor :type Actor%20Object%20Reference))
  (Variables|Default|SetIsOverlapping false))

(fn ConstructionScript
  (Transformation|SetActorRotation "0,135.000000, 0"))

(fn CheckifFalling)