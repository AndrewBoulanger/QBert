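; BP_Coily is the Coily enemy in a Q*bert-style game, hopping diagonally across cubes in pursuit of the player pawn.
; SettingTarget feeds the player's row and column to SetTargetRowAndCol.
; BeginPlay stores JumpTimeline at double speed, and its direction-specific tracks drive JumpLerp.
; Cube overlaps decide whether a finished jump plays the landing sound or starts falling, with a row/column bounds check triggering the fall sound.
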(event EventBeginPlay
  (bind _output_get (Variables|Default|SetTimeline (Variables|Default|GetJumpTimeline)))
  (Components|Timeline|SetPlayRate _output_get 2.0)
  (bind _asbp_player_pawn (Utilities|Casting|CastToBP_playerPawn (Game|Player|GetPlayerPawn 0)))
  (Variables|Default|SetQbert _asbp_player_pawn)
  (bind _returnvalue (Actor|GetActorOfClass "/Game/blueprints/BP_EnemySpawner.BP_EnemySpawner_C"))
  (Variables|Default|SetSpawner _returnvalue))

(event Collision|EventActorBeginOverlap
  (params (OtherActor :type Actor%20Object%20Reference))
  (if (Actor|ActorHasTag OtherActor "Cube")
    (Variables|Default|SetIsOverlapping true)
    (Class|Coily|StopFalling)))

(event EventTick
  (params (DeltaSeconds :type Float%20%28single-precision%29)))

(event Collision|EventActorEndOverlap
  (params (OtherActor :type Actor%20Object%20Reference))
  (Variables|Default|SetIsOverlapping false))

(event EventSettingTarget
  (bind _qbert (Variables|Default|GetQbert)
    (:then
      _)
    (:else
      (bind _asbp_player_pawn (Utilities|Casting|CastToBP_playerPawn (Game|Player|GetPlayerPawn 0)))
      (Variables|Default|SetQbert _asbp_player_pawn)))
  (Class|Coily|SetTargetRowandCol (Variables|/Script/QBert.playerPawn|Getm_row _qbert) (Variables|/Script/QBert.playerPawn|Getm_column _qbert)))

(fn ConstructionScript
  (Transformation|SetActorRotation "0,135.000000, 0"))

(fn CheckifFalling
  (if (or (< (Variables|Default|Getm_col) 1) (> (Variables|Default|Getm_col) (Variables|Default|Getm_row)))
    (Audio|Components|Audio|Play (Variables|Default|GetCoilyFall) 0.0)))