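; BP_saveGame is a save game Blueprint that stores a ranked top-ten list of high scores.
; AddScore inserts a new entry above the first lower score, drops the entry pushed past tenth place, and ignores scores that do not qualify.
; On a successful insert, it copies the list into a freshly created save object and writes that to the "BP_saveGame" slot.
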(fn AddScore
  (params (highScore :type Score%20Structure))
  (LocalVariables|Setnew_score highScore)
  (for _index (range 0 9)
    (if (> (.Score (Utilities|Struct|BreakScore (LocalVariables|Getnew_score))) (.Score (Utilities|Struct|BreakScore (Utilities|Array|Get(acopy) (Variables|Default|Getscores) _index))))
      (Utilities|Array|Insert (Variables|Default|Getscores) (LocalVariables|Getnew_score) _index)
      (Utilities|Array|RemoveIndex (Variables|Default|Getscores) 10)
      (bind _returnvalue (SaveGame|CreateSaveGameObject "BP_saveGame_C"))
      (Variables|BP_saveGame_C|Setscores _returnvalue (Variables|Default|Getscores))
      (SaveGame|SaveGametoSlot _returnvalue "BP_saveGame")
      (return))))