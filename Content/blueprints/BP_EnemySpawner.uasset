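; Enemy spawner for a Q*bert-style game that serves enemies from an object pool and manages a single reusable Coily egg.
; On BeginPlay it pre-spawns a shuffled pool of base enemies and green blobs, plus the egg, then respawns them at requested locations.
; DeleteEnemies moves dead enemies from the active list back to inactive.
; Coily's death deactivates all active enemies and awards score through the game mode; PauseEnemies is an empty stub.
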(event EventBeginPlay
  (CallFunction|PopulatePool)
  (bind _returnvalue (Game|SpawnActorfromClass "/Game/blueprints/BP_CoilyEgg.BP_CoilyEgg_C" (Variables|Default|GetBasicTransform) "Undefined" self 0))
  (Variables|Default|SetCoilyEgg _returnvalue))

(event Collision|EventActorBeginOverlap
  (params (OtherActor :type Actor%20Object%20Reference)))

(event EventSpawnEnemy
  (params (location :type Vector :default "0, 0, 0"))
  (bind _newenemy (CallFunction|PopQueue))
  (Class|BaseEnemy|Respawn _newenemy location))

(event EventSpawnCoilyEgg
  (params (location :type Vector :default "0, 0, 0"))
  (Class|BaseEnemy|Respawn (Variables|Default|GetCoilyEgg) location))

(event EventDeleteEnemies
  (CallFunction|ReturntoInactive))

(event EventCoilyDeath
  (CallFunction|ReturnAll)
  (bind _asbp_qbert_game_mode (Utilities|Casting|CastToBP_QBertGameMode (Game|GetGameMode)))
  (Class|QBertGameModeBase|RaiseScore _asbp_qbert_game_mode 500))

(fn ConstructionScript)

(fn PopulatePool
  (bind _inactive (Variables|Default|Getinactive))
  (for _index (range 0 18)
    (bind _returnvalue (Game|SpawnActorfromClass "/Game/blueprints/BP_BaseEnemy.BP_BaseEnemy_C" (Variables|Default|GetBasicTransform) "Undefined" self 0))
    (Utilities|Array|Add _inactive _returnvalue))
  (for _index_2 (range 0 3)
    (bind _returnvalue_2 (Game|SpawnActorfromClass "/Game/blueprints/BP_GreenBlob.BP_GreenBlob_C" (Variables|Default|GetBasicTransform) "Undefined" self 0))
    (Utilities|Array|Add _inactive _returnvalue_2))
  (Utilities|Array|Shuffle (Variables|Default|Getinactive)))

(fn PopQueue
  (LocalVariables|SetEnemy (Utilities|Array|Get(acopy) (Variables|Default|Getinactive)))
  (bind _enemy (LocalVariables|GetEnemy)
    (:then
      (Utilities|Array|Add (Variables|Default|GetActive) _enemy)
      (Utilities|Array|RemoveIndex (Variables|Default|Getinactive))
      (return (LocalVariables|GetEnemy)))
    (:else)))

(fn ReturntoInactive
  (for _index (range 0 (Utilities|Array|LastIndex (Variables|Default|GetActive)))
    (bind _returnvalue (Class|BaseEnemy|GetIsDead (Utilities|Array|Get(acopy) (Variables|Default|GetActive) _index)))
    (if _returnvalue
      (Utilities|Array|Add (Variables|Default|Getinactive) (Utilities|Array|Get(acopy) (Variables|Default|GetActive) _index))
      (Utilities|Array|RemoveIndex (Variables|Default|GetActive) _index))))

(fn ReturnAll
  (for _index (range 0 (Utilities|Array|LastIndex (Variables|Default|GetActive)))
    (Variables|/Script/QBert.BaseEnemy|SetreadyToDie (Utilities|Array|Get(acopy) (Variables|Default|GetActive) _index) true)
    (Class|BaseEnemy|SetActive (Utilities|Array|Get(acopy) (Variables|Default|GetActive) _index) false)))

(fn PauseEnemies
  (params (pauseTime :type Float%20%28single-precision%29)))