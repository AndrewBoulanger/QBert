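; Q*bert elevator actor that carries the player pawn along an InterpToMovement path once the pawn overlaps it.
; On overlap it sets the pawn falling with a rotating flipbook, toggles its disabled state, attaches it, plays the lift sound and starts the movement.
; When movement stops at world X zero, it detaches the pawn, resets its row and column, decrements the game mode's elevators and destroys itself.
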(event OnInterptoStop(InterpToMovement)
  (params (ImpactResult :type Hit%20Result%20Structure%20%28by%20ref%29) (Time :type Float%20%28single-precision%29))
  (Collision|SetActorEnableCollision false)
  (if (== (.x (Transformation|GetActorLocation)) 0.0)
    (Utilities|IsValid (Variables|Default|GetQBert)
      (:Is%20Valid
        (Transformation|DetachFromActor (Variables|Default|GetQBert) "KeepWorld" "KeepWorld" "KeepWorld")
        (Default|ToggleDisabled (Variables|Default|GetQBert) true)
        (Variables|/Script/QBert.playerPawn|SetisFalling (Variables|Default|GetQBert) true)
        (Class|PlayerPawn|ResetRowandColumn (Variables|Default|GetQBert))
        (bind _asbp_qbert_game_mode (Utilities|Casting|CastToBP_QBertGameMode (Game|GetGameMode)))
        (Class|QBertGameModeBase|ReduceElevators _asbp_qbert_game_mode)
        (Actor|DestroyActor)))))

(event EventBeginPlay
  (|CallParentFunction)
  (Class|Actor|SetTickablewhenPaused true)
  (Class|ActorComponent|SetTickablewhenPaused (Variables|Default|GetElevatorSprite) true))

(event Collision|EventActorBeginOverlap
  (params (OtherActor :type Actor%20Object%20Reference))
  (bind _asbp_player_pawn (Utilities|Casting|CastToBP_playerPawn OtherActor))
  (bind _output_get (Variables|Default|SetQBert _asbp_player_pawn))
  (Variables|/Script/QBert.playerPawn|SetisFalling _output_get true)
  (Sprite|SetFlipbook (Variables|/Script/QBert.playerPawn|GetSprites _output_get) "/Game/sprites/rotating.rotating")
  (Components|Timeline|PlayfromStart (Variables|/Script/QBert.playerPawn|GetSprites _output_get))
  (Default|ToggleDisabled (Variables|Default|GetQBert) false)
  (Transformation|AttachActorToActor (Variables|Default|GetQBert) self "None" "KeepWorld" "KeepWorld" "KeepWorld" true)
  (Audio|Components|Audio|Play (Variables|Default|GetliftSound) 1.8)
  (Class|InterptoMovementComponent|FinaliseControlPoints (Variables|Default|GetInterpToMovement))
  (Components|Activation|Activate (Variables|Default|GetInterpToMovement) true))

(event EventTick
  (params (DeltaSeconds :type Float%20%28single-precision%29)))

(fn ConstructionScript
  (|CallParentFunction))