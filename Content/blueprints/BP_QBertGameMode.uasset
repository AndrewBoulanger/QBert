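; Game mode for a Q*bert game that handles winning, game over and HUD updates.
; UpdateUI pushes score and lives to the widget.
; OnWin pauses, plays the win tune, then awards a completion bonus plus points per active elevator before triggering game over.
; OnGameOver compares the score with the tenth entry in the saved score table, opening high-score entry if beaten, otherwise loading the main menu.
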(event EventBeginPlay
  (Class|Actor|SetTickablewhenPaused true))

(event EventTick
  (params (DeltaSeconds :type Float%20%28single-precision%29)))

(event EventOnWin
  (params (duration :type Float%20%28single-precision%29))
  (Audio|Components|Audio|Play (Variables|Default|GetwinTune) 0.0)
  (Class|Actor|SetTickablewhenPaused true)
  (Game|SetGamePaused true)
  (Utilities|FlowControl|Delay (Variables|Default|GetsongDuration))
  (Class|QBertGameModeBase|RaiseScore (+ (* (Variables|Default|GetactiveElevators) 100) 1000))
  (Class|QBertGameModeBase|OnGameOver))

(event EventOnGameOver
  (bind _returnvalue (Game|GetPlayerController 0))
  (bind _returnvalue_2 (SaveGame|LoadGamefromSlot "BP_saveGame"))
  (bind _asbp_save_game (Utilities|Casting|CastToBP_saveGame _returnvalue_2))
  (Game|SetGamePaused true)
  (Utilities|FlowControl|Delay 2.0)
  (bind _returnvalue_3 (Class|QBertGameModeBase|GetScore))
  (if (> _returnvalue_3 (.Score (Utilities|Struct|BreakScore (Utilities|Array|Get(acopy) (Variables|/Game/blueprints/BP_saveGame.BP_saveGame_C|Getscores _asbp_save_game) 9))))
    (Viewport|RemoveAllWidgets)
    (bind _returnvalue_4 (UserInterface|CreateWidget "/Game/blueprints/SetHighScore_Widget.SetHighScore_Widget_C"))
    (Variables|/Game/blueprints/SetHighScore_Widget.SetHighScore_Widget_C|SetnewScore _returnvalue_4 _returnvalue_3)
    (UserInterface|Viewport|AddtoViewport _returnvalue_4 0)
    (Input|SetInputModeUIOnly _returnvalue _returnvalue_4 "DoNotLock")
    (Variables|/Script/Engine.PlayerController|SetbShowMouseCursor _returnvalue true)
    (Game|SetGamePaused true)
    (else
      (Game|OpenLevel(byName) "MainMenu"))))

(event EventUpdateUI
  (Variables|Default|GetUi
    (:then
      (bind _returnvalue (Class|QBertGameModeBase|GetLives))
      (bind _returnvalue_2 (Class|QBertGameModeBase|GetScore))
      (Default|UpdateData (Variables|Default|GetUi) _returnvalue_2 _returnvalue))
    (:else
      (bind _foundwidgets (Widget|GetAllWidgetsOfClass "/Game/blueprints/UI_widget.UI_widget_C" true)))))

(fn ConstructionScript)