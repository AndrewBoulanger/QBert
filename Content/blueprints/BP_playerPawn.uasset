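; Player pawn for a Q*bert-style game, handling cube landings, falls, pickups and enemy hits.
; Tag-based overlaps light cubes, set elevator fall rate, or trigger green-blob score and a five-second time freeze using pause-exempt ticking.
; Enemy hits cost a life, show a swear actor, briefly pause, then clear enemies through the spawner.
; JumpTimeline handlers define directional hops and row/column fall sounds; the timeline is stored at BeginPlay.
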(event EventBeginPlay
  (Components|Timeline|SetPlayRate (Variables|Default|GetjumpTimeline) 1.5)
  (Variables|Default|SetTimeline (Variables|Default|GetjumpTimeline))
  (bind _returnvalue (Game|SpawnActorfromClass "/Game/blueprints/BP_swear.BP_swear_C" (Transformation|GetActorTransform) "Undefined" 0 0))
  (Variables|Default|SetSwear _returnvalue)
  (bind _returnvalue_2 (Actor|GetActorOfClass "/Game/blueprints/BP_EnemySpawner.BP_EnemySpawner_C"))
  (Variables|Default|Setspawner _returnvalue_2)
  (Class|ActorComponent|SetTickablewhenPaused (Variables|Default|GetSprites) true))

(event Collision|EventActorBeginOverlap
  (params (OtherActor :type Actor%20Object%20Reference))
  (bind _returnvalue (Class|GameplayStatics|GetPlayerControllerfromID))
  (Variables|Default|SetIsOverlapping true)
  (switch name (Utilities|Array|Get(acopy) (Variables|/Script/Engine.Actor|GetTags OtherActor))
    (:Cube
      (bind _ascube_blueprint (Utilities|Casting|CastToCube_Blueprint OtherActor))
      (Variables|Default|SetCube _ascube_blueprint)
      (if (Variables|Default|GetisFalling)
        (Default|TurnLightonEvent (Variables|Default|GetCube)))
      (Variables|Default|SetisFalling false))
    (:points
      (Class|QBertGameModeBase|RaiseScore (Variables|Default|GetgameMode) 100)
      (bind _asbp_green_blob (Utilities|Casting|CastToBP_GreenBlob OtherActor))
      (Variables|/Script/QBert.BaseEnemy|SetreadyToDie _asbp_green_blob true)
      (Audio|Components|Audio|Play (Variables|Default|GettimeFreezeSound) 0.0)
      (Class|BaseEnemy|SetActive _asbp_green_blob false)
      (Class|Actor|SetTickablewhenPaused true)
      (Variables|/Script/Engine.PlayerController|SetbShouldPerformFullTickWhenPaused _returnvalue true)
      (Input|EnableInput _returnvalue)
      (Class|ActorComponent|SetTickablewhenPaused (Variables|Default|GetjumpTimeline) true)
      (Game|SetGamePaused true)
      (Utilities|FlowControl|Delay 5.0)
      (Game|SetGamePaused false)
      (Class|Actor|SetTickablewhenPaused false)
      (Class|ActorComponent|SetTickablewhenPaused (Variables|Default|GetjumpTimeline) false)
      (Audio|Components|Audio|Stop (Variables|Default|GettimeFreezeSound)))
    (:enemy
      (CallFunction|EnemyCollision))
    (:Elevator
      (Variables|Default|SetfallRate 3e+02))))

(event EventTick
  (params (DeltaSeconds :type Float%20%28single-precision%29)))

(event EventOnDelay
  (Utilities|FlowControl|Delay 1.0)
  (Transformation|SetActorLocation "0, 0, 0" false true)
  (bind _asbp_qbert_game_mode (Utilities|Casting|CastToBP_QBertGameMode (Game|GetGameMode)))
  (Class|QBertGameModeBase|LoseLife _asbp_qbert_game_mode))

(event Collision|EventActorEndOverlap
  (params (OtherActor :type Actor%20Object%20Reference))
  (Variables|Default|SetIsOverlapping false))

(event EventResetEnemies
  (Class|Actor|SetTickablewhenPaused true)
  (Game|SetGamePaused true)
  (Utilities|FlowControl|Delay 1.0)
  (CallFunction|Reset)
  (Class|Actor|SetTickablewhenPaused false))

(fn ConstructionScript)

(fn Reset
  (Game|SetGamePaused false)
  (Default|ReturnAll (Variables|Default|Getspawner))
  (bind _returnvalue (Actor|GetActorOfClass "/Game/blueprints/BP_Coily.BP_Coily_C"))
  (Class|Coily|SetActive _returnvalue false)
  (bind _returnvalue_2 (Actor|GetActorOfClass "/Game/blueprints/BP_CoilyEgg.BP_CoilyEgg_C"))
  (Class|BaseEnemy|SetActive _returnvalue_2 false)
  (Variables|/Script/QBert.BaseEnemy|SetreadyToDie _returnvalue_2 true)
  (Class|EnemySpawner|ResetSpawns (Variables|Default|Getspawner)))

(fn EnemyCollision
  (Audio|Components|Audio|Play (Variables|Default|GetswearSound) 0.0)
  (Class|QBertGameModeBase|LoseLife (Variables|Default|GetgameMode))
  (Default|Spawnin (Variables|Default|GetSwear) (+ (Transformation|GetActorLocation) "-50.000000,-50.000000,100.000000"))
  (Class|PlayerPawn|ResetEnemies))

(fn ToggleDisabled
  (params (enabled :type Boolean))
  (Actor|Tick|SetActorTickEnabled enabled)
  (Collision|SetActorEnableCollision enabled))

(fn CheckifFalling
  (if (and (Math|Boolean|ORBoolean (> (Variables|Default|Getm_row) 7) (< (Variables|Default|Getm_column) 1) (> (Variables|Default|Getm_column) (Variables|Default|Getm_row))) (!= (Variables|Default|Getm_row) 5))
    (if (not (Variables|Default|GetIsOverlapping))
      (Audio|Components|Audio|Play (Variables|Default|GetQbertFall) 0.0))
    (else
      (Audio|Components|Audio|Play (Variables|Default|GetQbertJump) 0.0))))