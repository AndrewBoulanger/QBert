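; BP_CoilyEgg is the Coily egg enemy, which tracks its position on the cube grid and hatches into Coily.
; BeginPlay pre-spawns an inactive BP_Coily, and overlaps with Cube_Blueprint update the egg's row and column.
; At row seven or beyond, the egg stops ticking and starts hatching.
; After a short delay, unless ReadyToDie, it spawns Coily in above itself, passes on its grid position and deactivates.
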(event Custom|Hatch_Event
  (Utilities|FlowControl|Delay 2.0)
  (if (not (Variables|Default|GetreadyToDie))
    (Class|Coily|Spawnin (Variables|Default|Getcoily) (+ (Transformation|GetActorLocation) "0, 0,50.000000"))
    (Class|Coily|SetRowandCol (Variables|Default|Getcoily) (Variables|Default|Getm_row) (Variables|Default|Getm_column))
    (Class|BaseEnemy|SetActive false)))

(event EventBeginPlay
  (|CallParentFunction)
  (bind _returnvalue (Game|SpawnActorfromClass "/Game/blueprints/BP_Coily.BP_Coily_C" (Transformation|GetActorTransform) "Undefined" 0 0))
  (bind _output_get (Variables|Default|Setcoily _returnvalue))
  (Class|Coily|SetActive _output_get false))

(event Collision|EventActorBeginOverlap
  (params (OtherActor :type Actor%20Object%20Reference))
  (|CallParentFunction OtherActor)
  (bind _ascube_blueprint (Utilities|Casting|CastToCube_Blueprint OtherActor))
  (CallFunction|UpdateLocation _ascube_blueprint))

(event EventTick
  (params (DeltaSeconds :type Float%20%28single-precision%29))
  (|CallParentFunction DeltaSeconds))

(fn ConstructionScript
  (|CallParentFunction))

(fn UpdateLocation
  (params (NewParam :type Cube%20Blueprint%20Object%20Reference))
  (Variables|Default|Setm_column (Variables|/Game/blueprints/Cube_Blueprint.Cube_Blueprint_C|GetColumn NewParam))
  (bind _output_get (Variables|Default|Setm_row (Variables|/Game/blueprints/Cube_Blueprint.Cube_Blueprint_C|Getlevel NewParam)))
  (if (>= _output_get 7)
    (Variables|Default|SetreadyToHatch true)
    (Actor|Tick|SetActorTickEnabled false)
    (CallFunction|HatchEvent)))