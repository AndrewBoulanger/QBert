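; Q*Bert platform cube that changes its top material when first turned on and reports to BP_QBertGameMode to reduce the remaining platform count.
; The construction script fixes its rotation and derives its height from Level.
; It binds to the game mode's game-won event, which seeds a timer that Tick counts down, alternating the two top materials by parity to flash, with ticking allowed while paused.
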(event Custom|OnGameWon_Event_0
  (params (duration :type Float%20%28single-precision%29))
  (Variables|Default|Setflashtimer duration)
  (Variables|Default|SetisFlashing true))

(event Custom|turnLightOn_Event
  (if (not (Variables|Default|GetIsOn))
    (Variables|Default|SetIsOn true)
    (Rendering|Material|SetMaterial (Variables|Default|GetPlane) 0 "/Game/material/top2.top2")
    (bind _asbp_qbert_game_mode (Utilities|Casting|CastToBP_QBertGameMode (Game|GetGameMode)))
    (Class|QBertGameModeBase|ReduceRemainingPlatforms _asbp_qbert_game_mode)))

(event EventBeginPlay
  (Class|Actor|SetTickablewhenPaused true)
  (bind _asbp_qbert_game_mode (Utilities|Casting|CastToBP_QBertGameMode (Game|GetGameMode)))
  (EventDispatchers|AssignOnGameWon _asbp_qbert_game_mode (delegate Custom|OnGameWon_Event_0)))

(event Collision|EventActorBeginOverlap
  (params (OtherActor :type Actor%20Object%20Reference)))

(event EventTick
  (params (DeltaSeconds :type Float%20%28single-precision%29))
  (if (Variables|Default|GetisFlashing)
    (bind _output_get (Variables|Default|Setflashtimer (- (Variables|Default|Getflashtimer) (* (Utilities|Time|GetWorldDeltaSeconds) 3.0))))
    (if (== (Math|Integer|%(Integer) (Math|Float|Truncate _output_get) 2) 0)
      (Rendering|Material|SetMaterial (Variables|Default|GetPlane) 0 "/Game/material/top2.top2")
      (else
        (Rendering|Material|SetMaterial (Variables|Default|GetPlane) 0 "/Game/material/top1.top1")))))

(fn ConstructionScript
  (bind _returnvalue (Transformation|GetActorLocation))
  (Transformation|SetActorRotation "0,90.000000, 0")
  (Transformation|SetActorLocation (Math|Vector|MakeVector (.x _returnvalue) (.y _returnvalue) (Math|Conversions|ToFloat(Integer) (* (Variables|Default|Getlevel) -80))) false false))

(fn FlashLights
  (params (duration :type Float%20%28single-precision%29)))