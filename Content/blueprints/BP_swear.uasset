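; BP_swear is a reusable actor that pops in at a given position and hides itself after a set lifetime.
; SpawnIn moves it, resets the timer and activates it; Tick counts down and calls SetActive to hide it and stop ticking.
; Toggling visibility and tick instead of spawning or destroying suits pooling.
; It keeps ticking while paused, and construction applies a fixed rotation.
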(event EventBeginPlay
  (Class|Actor|SetTickablewhenPaused true))

(event Collision|EventActorBeginOverlap
  (params (OtherActor :type Actor%20Object%20Reference)))

(event EventTick
  (params (DeltaSeconds :type Float%20%28single-precision%29))
  (bind _output_get (Variables|Default|SetTimer (- (Variables|Default|GetTimer) DeltaSeconds)))
  (if (<= _output_get 0.0)
    (CallFunction|SetActive false)))

(fn ConstructionScript
  (Transformation|SetActorRotation "0,135.000000, 0"))

(fn SetActive
  (params (isActive :type Boolean))
  (bind _output_get (LocalVariables|SetActive isActive))
  (Rendering|SetActorHiddenInGame (not _output_get))
  (Actor|Tick|SetActorTickEnabled (LocalVariables|GetActive)))

(fn Spawnin
  (params (pos :type Vector))
  (Transformation|SetActorLocation pos false false)
  (Variables|Default|SetTimer (Variables|Default|GetlifeTime))
  (CallFunction|SetActive true))